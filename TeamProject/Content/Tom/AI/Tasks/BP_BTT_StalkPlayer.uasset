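; Behavior tree task that makes the mannequin AI stalk the player by moving to a nearby spot hidden from them.
; It gets the player through a pawn message and picks a random reachable point within a radius around them.
; A visibility trace to the player, ignoring the player, must be blocked for the move to start.
; The task succeeds on arrival and fails on a clear trace or failed move, without retrying.
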(event `self.ReceiveExecuteAI`
  (params (OwnerController :type "AIController Object Reference") (ControlledPawn :type "Pawn Object Reference"))
  (bind _actors_to_ignore (`self.Actors to Ignore`))
  (bind _mannequinneref (message `/Game/Tom/Tom_Blueprints/BPI_GetEnemy.GetThingFromPawn` ControlledPawn))
  (bind _output_get (set `self.Mannequinne Ref` _mannequinneref))
  (bind _output_get_2 (set `self.Player Ref` (`/Game/Sharan/Blueprints/RBP_Mannequine1.GetPlayerRef` _output_get)))
  (`KismetArrayLibrary.Array_Add` _actors_to_ignore)
  (`KismetArrayLibrary.Array_Add` _actors_to_ignore _output_get_2)
  (bind _output_get_3 (set `self.LocationToMoveTo` (`NavigationSystemV1.K2_GetRandomReachablePointInRadius` (`Actor.K2_GetActorLocation` (`self.Player Ref`)) 1000.0 null null)))
  (bind (_outhit _returnvalue) (`KismetSystemLibrary.LineTraceSingle` _output_get_3 (`Actor.K2_GetActorLocation` (`self.Player Ref`)) "TraceTypeQuery1" false (`self.Actors to Ignore`)))
  (if _returnvalue
    (`|AIMoveTo` ControlledPawn (`self.LocationToMoveTo`) null
      (:`OnSuccess`
        (`self.FinishExecute` true))
      (:`OnFail`
        (`self.FinishExecute` false)))
    (else
      (`self.FinishExecute` false))))