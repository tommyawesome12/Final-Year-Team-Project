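; Behavior tree task that copies the player's sanity into a blackboard float for the mannequin AI.
; On AI execute, it checks that the controlled pawn implements BPI_GetEnemy and uses that interface to get the mannequin reference.
; It then reads Sanity from the mannequin's player reference, writes it to the blackboard key and finishes successfully.
; Pawns without the interface trigger FinishAbort instead of a failed finish.
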(event `self.ReceiveExecuteAI`
  (params (OwnerController :type "AIController Object Reference") (ControlledPawn :type "Pawn Object Reference"))
  (if (`KismetSystemLibrary.DoesImplementInterface` ControlledPawn "/Game/Tom/Tom_Blueprints/BPI_GetEnemy.BPI_GetEnemy_C")
    (bind _mannequinneref (message `/Game/Tom/Tom_Blueprints/BPI_GetEnemy.GetThingFromPawn` ControlledPawn))
    (bind _output_get (set `self.MannequineRef` _mannequinneref))
    (bind _output_get_2 (set `self.PlayerRef` (`/Game/Tom/AI/BP_AITest.GetPlayerRef` _output_get)))
    (`BTFunctionLibrary.SetBlackboardValueAsFloat` (`self.BlackoardRef`) (`/Game/Tom/Tom_Blueprints/BP_PlayerCharacter.Sanity` _output_get_2))
    (`self.FinishExecute` true)
    (else
      (`self.FinishAbort`))))