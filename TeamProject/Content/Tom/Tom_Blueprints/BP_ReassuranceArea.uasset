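; Reassurance area actor that gives the player a temporary safe spot under a warm spotlight, then destroys itself once used up.
; While the player overlaps its box, a line trace checks for blockers; clear sight clears InBadPlace on the Level 1 game mode and messages the player.
; Safe time advances a timer that dims the light.
; The construction script adds the mesh and spotlight, compensating for actor scale.
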(event `self.ReceiveBeginPlay`
  (bind _actors_to_ignore (`self.Actors to Ignore`))
  ;[1 1 1] Sets variable
  (bind _asbp_gm_level_1 (cast `/Game/Tom/Tom_Blueprints/BP_GM_Level1` (`GameplayStatics.GetGameMode`)))
  (set `self.GameModeRef` _asbp_gm_level_1)
  (`KismetArrayLibrary.Array_Add` _actors_to_ignore self)
  (`KismetArrayLibrary.Array_Add` _actors_to_ignore (`GameplayStatics.GetPlayerCharacter` 0)))

(event `self.ReceiveTick`
  (params (DeltaSeconds :type "Float (single-precision)"))
  (bind _gamemoderef (`self.GameModeRef`))
  (if (>= (`self.Timer`) (`self.Duration`))
    (`self.K2_DestroyActor`)
    (else
      ;[1 1 1] Checks that there is no wall in the way
      (if (`self.playerInRange`)
        (`|ExecutionSequence`
          (:`then_0`
            (bind (_outhit _returnvalue) (`KismetSystemLibrary.LineTraceSingle` (`self.K2_GetActorLocation`) (`self.K2_GetActorLocation` (`GameplayStatics.GetPlayerCharacter` 0)) "TraceTypeQuery3" false (`self.Actors to Ignore`)))
            (if _returnvalue
              (set `/Game/Tom/Tom_Blueprints/BP_GM_Level1.InBadPlace` true _gamemoderef)
              (else
                (set `/Game/Tom/Tom_Blueprints/BP_GM_Level1.InBadPlace` false _gamemoderef)
                (message `/Game/Tom/Tom_Blueprints/BPI_ReassuranceInterface.ReassuranceAreaEnter` (`self.TargetPlayer`) self))))
          (:`then_1`
            ;[1 1 1] timer for duraion
            (if (not (`/Game/Tom/Tom_Blueprints/BP_GM_Level1.InBadPlace` (`self.GameModeRef`)))
              (set `self.Timer` (+ DeltaSeconds (`self.Timer`)))))
          (:`then_2`
            (`LightComponent.SetIntensity` (`self.LightRef`) (* (- 1.0 (/ (`self.Timer`) (`self.Duration`))) 50000.0))))))))

(event `self.Box.OnComponentBeginOverlap`
  (params (OverlappedComponent :type "PrimitiveComponent Object Reference") (OtherActor :type "Actor Object Reference") (OtherComp :type "PrimitiveComponent Object Reference") (OtherBodyIndex :type Integer) (bFromSweep :type Boolean) (SweepResult :type "HitResult Structure (by ref)"))
  ;[1 1 1] Chekcs if player is inside colision or not
  (set `self.TargetPlayer` OtherActor)
  (if (`self.ActorHasTag` OtherActor "Player")
    (set `self.playerInRange` true)))

(event `self.Box.OnComponentEndOverlap`
  (params (OverlappedComponent :type "PrimitiveComponent Object Reference") (OtherActor :type "Actor Object Reference") (OtherComp :type "PrimitiveComponent Object Reference") (OtherBodyIndex :type Integer))
  ;[1 1 1] Chekcs if player is inside colision or not
  (set `self.TargetPlayer` null)
  (if (`self.ActorHasTag` OtherActor "Player")
    (set `self.playerInRange` false)
    (set `/Game/Tom/Tom_Blueprints/BP_GM_Level1.InBadPlace` true (`self.GameModeRef`))
    (message `/Game/Tom/Tom_Blueprints/BPI_ReassuranceInterface.ReassuranceAreaExit` OtherActor)))

(fn `UserConstructionScript`
  (bind (_returnvalue_x _returnvalue_y _returnvalue_z) (`KismetMathLibrary.BreakVector` (`self.GetActorScale3D`)))
  (bind _returnvalue (`AddComponent|NODE_AddSkeletalMeshComponent-0` :`RelativeTransform` (`KismetMathLibrary.MakeTransform` (`KismetMathLibrary.MakeVector` 0.0 0.0 (/ -100.0 _returnvalue_z)) (struct) (`KismetMathLibrary.MakeVector` (/ 1.0 _returnvalue_x) (/ 1.0 _returnvalue_y) (/ 1.0 _returnvalue_z)))))
  (`SkeletalMeshComponent.SetSkeletalMeshAsset` _returnvalue "/Engine/Tutorial/SubEditors/TutorialAssets/Character/TutorialTPP.TutorialTPP")
  (bind _returnvalue_2 (`AddComponent|NODE_AddSpotLightComponent-0` :`RelativeTransform` (`KismetMathLibrary.MakeTransform` (`KismetMathLibrary.MakeVector` 0.0 0.0 (/ 600.0 _returnvalue_z)) (struct :`Pitch` -90.0))))
  (set `self.LightRef` _returnvalue_2)
  (`LightComponent.SetIntensity` _returnvalue_2 50000.0)
  (`LightComponent.SetLightColor` _returnvalue_2 (struct :`R` 1.0 :`G` 0.743638 :`B` 0.125 :`A` 1.0) true))