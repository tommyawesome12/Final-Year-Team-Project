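; BP_FoldedTrousers is a folded trousers prop whose material changes appearance with a sanity value.
; The construction script builds a dynamic material with good and bad base colour, ORM and normal textures, plus a random colour.
; BeginPlay resets Sanity to a midpoint.
; UpdateTexture offsets and clamps incoming sanity to drive the Sanity parameter and replace RandomColour with a grey-to-black blend.
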(event `self.ReceiveBeginPlay`
  (`MaterialInstanceDynamic.SetScalarParameterValue` (`self.DynamicMaterialInstance`) "Sanity" 0.5))

(event `UpdateTexture`
  (params (SanityValue :type "Float (double-precision)"))
  (bind _dynamicmaterialinstance (`self.DynamicMaterialInstance`))
  (bind _returnvalue (`KismetMathLibrary.FClamp` (- SanityValue 0.5)))
  (if true
    (`MaterialInstanceDynamic.SetScalarParameterValue` _dynamicmaterialinstance "Sanity" _returnvalue)
    (`MaterialInstanceDynamic.SetVectorParameterValue` _dynamicmaterialinstance "RandomColour" (`KismetMathLibrary.LinearColorLerp` (struct :`R` 0.375 :`G` 0.375 :`B` 0.375 :`A` 1.0) (struct) _returnvalue))))

(fn `UserConstructionScript`
  (bind _returnvalue (`KismetMaterialLibrary.CreateDynamicMaterialInstance` (`self.MaterialInstace`)))
  (set `self.DynamicMaterialInstance` _returnvalue)
  (`MaterialInstanceDynamic.SetTextureParameterValue` _returnvalue "GoodTextureBaseColour" (`self.GoodTextureBaseColour`))
  (`MaterialInstanceDynamic.SetTextureParameterValue` _returnvalue "BadTextureBaseColour" (`self.BadTextureBaseColour`))
  (`MaterialInstanceDynamic.SetTextureParameterValue` _returnvalue "GoodTextureORM" (`self.GoodTextureORM`))
  (`MaterialInstanceDynamic.SetTextureParameterValue` _returnvalue "BadTextureORM" (`self.BadTextureORM`))
  (`MaterialInstanceDynamic.SetTextureParameterValue` _returnvalue "GoodTextureNormal" (`self.GoodTextureNormal`))
  (`MaterialInstanceDynamic.SetTextureParameterValue` _returnvalue "BadTextureNormal" (`self.BadTextureNormal`))
  (`MaterialInstanceDynamic.SetScalarParameterValue` _returnvalue "Sanity" 1.0)
  (bind _output_get (set `self.LinearColour` (make `LinearColor` (`KismetMathLibrary.RandomFloat`) (`KismetMathLibrary.RandomFloat`) (`KismetMathLibrary.RandomFloat`) 1.0)))
  (`MaterialInstanceDynamic.SetVectorParameterValue` (`self.DynamicMaterialInstance`) "RandomColour" _output_get)
  (`PrimitiveComponent.SetMaterial` (`self.StaticMesh`) 0 _returnvalue))