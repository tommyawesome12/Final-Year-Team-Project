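; BP_FollowCamera is a camera actor that tracks the player and can fall, turning into a projectile.
; It finds BP_PlayerCharacter on BeginPlay, then rotates its Arrow component toward the player every Tick unless Fallen is set.
; The Fall event hides CameraPart and its children and spawns a BP_CameraProjectile just below the actor, aimed at the player.
; Fallen is never set within this graph.
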(event `self.ReceiveBeginPlay`
  (bind _returnvalue (`GameplayStatics.GetActorOfClass` "/Game/Tom/Tom_Blueprints/BP_PlayerCharacter.BP_PlayerCharacter_C"))
  (set `self.PlayerRef` _returnvalue))

(event `self.ReceiveTick`
  (params (DeltaSeconds :type "Float (single-precision)"))
  (if (not (`self.Fallen`))
    (`SceneComponent.K2_SetWorldRotation` (`self.Arrow`) (`KismetMathLibrary.FindLookAtRotation` (`SceneComponent.K2_GetComponentLocation` (`self.Arrow`)) (`self.K2_GetActorLocation` (`self.PlayerRef`))) false false)))

(event `Fall`
  (`SceneComponent.SetHiddenInGame` (`self.CameraPart`) true true)
  (`|SpawnActorFromClass` "/Game/Tom/Tom_Blueprints/BP_CameraProjectile.BP_CameraProjectile_C" (`KismetMathLibrary.MakeTransform` (- (`self.K2_GetActorLocation`) (0.0 0.0 50.0)) (`KismetMathLibrary.FindLookAtRotation` (`SceneComponent.K2_GetComponentLocation` (`self.Arrow`)) (`self.K2_GetActorLocation` (`self.PlayerRef`)))) "Undefined" "MultiplyWithRoot" null null))

(fn `UserConstructionScript`)