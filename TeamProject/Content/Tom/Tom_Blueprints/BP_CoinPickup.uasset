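; BP_CoinPickup is a coin pickup that adds to the player's coin count.
; Its Interact event increments Coins on the passed player reference, then destroys the actor.
; The construction script calls the parent's, then sets MeshToUse to a machine coin mesh.
; Overlap and Tick events are disabled, so collection happens only through Interact.
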(event `self.ReceiveBeginPlay`
  (`parent.ReceiveBeginPlay`))

(event `/Game/Tom/Tom_Blueprints/BPI_Interact.Interact`
  (params (PlayerRef :type "/Game/Tom/Tom_Blueprints/BP_PlayerCharacter Object Reference"))
  (`/Engine/EditorBlueprintResources/StandardMacros.IncrementInt` (`/Game/Tom/Tom_Blueprints/BP_PlayerCharacter.Coins` PlayerRef)
    (:`  `
      (`self.K2_DestroyActor`))))

(fn `UserConstructionScript`
  (`parent.UserConstructionScript`)
  (set `self.MeshToUse` "/Game/Tom/ModelsAndTextures/Coin/SM_MachineCoin__1_.SM_MachineCoin__1_"))