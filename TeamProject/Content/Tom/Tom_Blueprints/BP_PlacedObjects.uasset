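; BP_PlacedObjects is a placeable mesh actor whose material responds to a sanity value, using a good and a bad texture.
; The construction script applies the configured mesh and creates a dynamic material instance with both textures and Sanity at full, assigned to the first material slot.
; UpdateTexture passes a new sanity value to that material's Sanity parameter at runtime.
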(event `UpdateTexture`
  (params (SanityValue :type "Float (double-precision)"))
  (if true
    (`MaterialInstanceDynamic.SetScalarParameterValue` (`self.DynamicMaterialInstance`) "Sanity" SanityValue)))

(fn `UserConstructionScript`
  (bind _staticmesh (`self.StaticMesh`))
  (`StaticMeshComponent.SetStaticMesh` _staticmesh (`self.Mesh`))
  (bind _returnvalue (`KismetMaterialLibrary.CreateDynamicMaterialInstance` (`self.MaterialInstace`)))
  (set `self.DynamicMaterialInstance` _returnvalue)
  (`MaterialInstanceDynamic.SetTextureParameterValue` _returnvalue "GoodTexture" (`self.GoodTexture`))
  (`MaterialInstanceDynamic.SetTextureParameterValue` _returnvalue "BadTexture" (`self.BadTexture`))
  (`MaterialInstanceDynamic.SetScalarParameterValue` _returnvalue "Sanity" 1.0)
  (`PrimitiveComponent.SetMaterial` _staticmesh 0 _returnvalue))