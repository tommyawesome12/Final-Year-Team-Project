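; Hiding place actor that moves the player in or out of hiding when interacted with.
; Interact reads the player's IsHiding flag, teleports player character 0 and flips the flag.
; The destination is the actor's location minus ExitLocation when hiding, or minus EntranceLocation when leaving.
; UseX picks whether only world X or Y changes, with the Y case using the offset's X component.
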(event `/Game/Tom/Tom_Blueprints/BPI_Interact.Interact`
  (params (PlayerRef :type "/Game/Tom/Tom_Blueprints/BP_PlayerCharacter Object Reference"))
  (bind _returnvalue (`GameplayStatics.GetPlayerCharacter` 0))
  (bind (_returnvalue_x _returnvalue_y _returnvalue_z) (`KismetMathLibrary.BreakVector` (`self.K2_GetActorLocation`)))
  (bind (_returnvalue_x_2 _returnvalue_y_2 _returnvalue_z_2) (`KismetMathLibrary.BreakVector` (`self.K2_GetActorLocation`)))
  (bind (_exitlocation_x _exitlocation_y _exitlocation_z) (`KismetMathLibrary.BreakVector` (`self.ExitLocation`)))
  (bind _player_ref (`self.Player Ref`))
  (bind _player_ref_2 (`self.Player Ref`))
  (bind (_entrancelocation_x _entrancelocation_y _entrancelocation_z) (`KismetMathLibrary.BreakVector` (`self.EntranceLocation`)))
  (bind (_returnvalue_x_3 _returnvalue_y_3 _returnvalue_z_3) (`KismetMathLibrary.BreakVector` (`self.K2_GetActorLocation` _returnvalue)))
  (bind _returnvalue_x_4 (`KismetMathLibrary.BreakVector` (- (`self.K2_GetActorLocation`) (`self.EntranceLocation`))))
  (bind (_returnvalue_x_5 _returnvalue_y_4) (`KismetMathLibrary.BreakVector` (- (`KismetMathLibrary.MakeVector` _returnvalue_x_2 _returnvalue_y_2 _returnvalue_z_2) (`KismetMathLibrary.MakeVector` _entrancelocation_y _entrancelocation_x _entrancelocation_z))))
  (bind (_returnvalue_x_6 _returnvalue_y_5) (`KismetMathLibrary.BreakVector` (- (`KismetMathLibrary.MakeVector` _returnvalue_x _returnvalue_y _returnvalue_z) (`KismetMathLibrary.MakeVector` _exitlocation_y _exitlocation_x _exitlocation_z))))
  (bind _returnvalue_x_7 (`KismetMathLibrary.BreakVector` (- (`self.K2_GetActorLocation`) (`self.ExitLocation`))))
  (bind _output_get (set `self.Player Ref` PlayerRef))
  (if (`/Game/Tom/Tom_Blueprints/BP_PlayerCharacter.IsHiding` _output_get)
    (if (`self.UseX`)
      (`self.K2_SetActorLocation` _returnvalue (`KismetMathLibrary.MakeVector` _returnvalue_x_4 _returnvalue_y_3 _returnvalue_z_3) false false)
      (set `/Game/Tom/Tom_Blueprints/BP_PlayerCharacter.IsHiding` false _player_ref_2)
      (else
        (`self.K2_SetActorLocation` _returnvalue (`KismetMathLibrary.MakeVector` _returnvalue_x_3 _returnvalue_y_4 _returnvalue_z_3) false false)
        (set `/Game/Tom/Tom_Blueprints/BP_PlayerCharacter.IsHiding` false _player_ref_2)))
    (elif (`self.UseX`)
      (`self.K2_SetActorLocation` _returnvalue (`KismetMathLibrary.MakeVector` _returnvalue_x_7 _returnvalue_y_3 _returnvalue_z_3) false false)
      (set `/Game/Tom/Tom_Blueprints/BP_PlayerCharacter.IsHiding` true _player_ref)
      (else
        (`self.K2_SetActorLocation` _returnvalue (`KismetMathLibrary.MakeVector` _returnvalue_x_3 _returnvalue_y_5 _returnvalue_z_3) false false)
        (set `/Game/Tom/Tom_Blueprints/BP_PlayerCharacter.IsHiding` true _player_ref)))))

(fn `UserConstructionScript`)