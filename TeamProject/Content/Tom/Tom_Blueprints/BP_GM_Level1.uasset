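; Level 1 game mode for a sanity-based horror level with dress, socks and boots objectives, reporting pickups to BP_Mother.
; BeginPlay caches level actors and spawns objectives and coins at random points, consuming each point and retrying recursively on failure.
; In the bad place, Tick drains sanity, which drives props, clothes racks, lighting, camera shake and blackout flickers synced to mannequins.
; Scare events are mostly stubs, and their random timer only prints.
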(event `self.ReceiveBeginPlay`
  (bind _outactors (`GameplayStatics.GetAllActorsOfClass` "/Game/Sharan/Blueprints/BP_Objectives.BP_Objectives_C"))
  (set `self.TotalItems` (`KismetArrayLibrary.Array_Length` _outactors))
  (bind _returnvalue (`GameplayStatics.GetActorOfClass` "/Game/Tom/Tom_Blueprints/BP_Mother.BP_Mother_C"))
  (set `self.MotherRef` _returnvalue)
  (bind _outactors_2 (`GameplayStatics.GetAllActorsOfClass` "/Game/Tom/Tom_Blueprints/BP_PlacedObjects.BP_PlacedObjects_C"))
  (set `self.PlacedObjectsArray` _outactors_2)
  (bind _outactors_3 (`GameplayStatics.GetAllActorsOfClass` "/Game/Tom/Tom_Blueprints/BP_Lights.BP_Lights_C"))
  (set `self.LightsVariable` _outactors_3)
  (bind _outactors_4 (`GameplayStatics.GetAllActorsOfClass` "/Game/Tom/Tom_Blueprints/BP_CothesRandomiser.BP_CothesRandomiser_C"))
  (set `self.ClothesRackArray` _outactors_4)
  (bind _outactors_5 (`GameplayStatics.GetAllActorsOfClass` "/Game/Tom/Tom_Blueprints/BP_HangerObjectiveSpawn.BP_HangerObjectiveSpawn_C"))
  (set `self.HangerSpawnPoints` _outactors_5)
  (bind _outactors_6 (`GameplayStatics.GetAllActorsOfClass` "/Game/Tom/Tom_Blueprints/BP_PigeonHoleObjectiveSpawn.BP_PigeonHoleObjectiveSpawn_C"))
  (set `self.PigeonHoleSpawnPoints` _outactors_6)
  (bind _returnvalue_2 (`GameplayStatics.GetActorOfClass` "/Game/Tom/Tom_Blueprints/BP_PlayerCharacter.BP_PlayerCharacter_C"))
  (set `self.PlayerRef` _returnvalue_2)
  (bind _outactors_7 (`GameplayStatics.GetAllActorsOfClass` "/Game/Sharan/Blueprints/RBP_Mannequine1.RBP_Mannequine1_C"))
  (set `self.ArrayOfMannequinnes` _outactors_7)
  (`self.Spawn Objectives`)
  (`self.EventGraphBeginPlay`)
  (`self.Spawn Coins`))

(event `self.ReceiveTick`
  (params (DeltaSeconds :type "Float (single-precision)"))
  (`self.SanityDrainOverTime` (/ DeltaSeconds (`self.Duration`)))
  (`self.EventGraphOnTick` DeltaSeconds)
  (if (`/Game/Tom/Tom_Blueprints/BP_PlayerCharacter.CanFadeToBlack` (`self.PlayerRef`))
    (if (`self.InBadPlace`)
      (`self.LightFlickering` DeltaSeconds))))

(event `Record Pickup`
  (params (Collected :type Integer))
  (bind _output_get (set `self.CollectedItems` Collected))
  (`/Game/Tom/Tom_Blueprints/BP_Mother.ItemCollected` (`self.MotherRef`) _output_get))

(event `SanityDrainOverTime`
  (params (DrainAmount :type "Float (double-precision)"))
  (if (`self.InBadPlace`)
    (`/Game/Tom/Tom_Blueprints/BP_PlayerCharacter.DecreaseSanity` (`self.PlayerRef`) DrainAmount)))

(event `UpdateSanity`
  (params (SanityValue :type "Float (double-precision)"))
  (`|ExecutionSequence`
    (:`then_0`
      (for _array_element (`self.PlacedObjectsArray`)
        (`/Game/Tom/Tom_Blueprints/BP_PlacedObjects.UpdateTexture` _array_element SanityValue)))
    (:`then_1`
      (for _array_element_2 (`self.ClothesRackArray`)
        (`/Game/Tom/Tom_Blueprints/BP_CothesRandomiser.UpdateClothes` _array_element_2 SanityValue)))
    (:`then_2`
      (if (<= SanityValue 0.1)
        (set `self.LightsFlicker` true)
        (else
          (set `self.LightsFlicker` false))))
    (:`then_3`
      (if (<= SanityValue 0.3)
        (`/Engine/EditorBlueprintResources/StandardMacros.DoOnce` false
          (:`Completed`
            (`GameplayStatics.PlayWorldCameraShake` "/Game/Tom/Tom_Blueprints/BP_CameraShake.BP_CameraShake_C" (`self.K2_GetActorLocation` (`self.PlayerRef`)) 0.0 300.0)))))
    (:`then_4`
      (for _array_element_3 (`self.LightsVariable`)
        (`/Game/Tom/Tom_Blueprints/BP_Lights.UpdateLighting` _array_element_3 SanityValue)))))

(event `UpdateMannequinneLoction`
  (for _array_element (`self.ArrayOfMannequinnes`)
    (`/Game/Sharan/Blueprints/RBP_Mannequine1.TeleportToStartPosition` _array_element)))

(event `LightFlickering`
  (params (TimeDelta :type "Float (double-precision)"))
  (bind _returnvalue (+ (`self.LightsTimer`) TimeDelta))
  ;[1 1 1] light flickering mechanic for when sanity is low enough
  (if (`self.LightsFlicker`)
    (if (`self.LightsOn`)
      (bind _output_get (set `self.LightsTimer` _returnvalue))
      (if (>= _output_get (`KismetMathLibrary.RandomFloatInRange` 2.0 5.0))
        (set `self.LightsOn` false)
        (set `self.LightsTimer` 0.0)
        (for _array_element (`self.LightsVariable`)
          (`/Game/Tom/Tom_Blueprints/BP_Lights.TurnLightOff` _array_element)
          (`/Game/Tom/Tom_Blueprints/BP_PlayerCharacter.FadeToBlack` (`self.PlayerRef`)))
        (for _array_element_2 (`self.ArrayOfMannequinnes`)
          (set `/Game/Sharan/Blueprints/RBP_Mannequine1.LightsOn` false _array_element_2)))
      (else
        (bind _output_get_2 (set `self.LightsTimer` _returnvalue))
        (if (>= _output_get_2 1.0)
          (set `self.LightsOn` true)
          (set `self.LightsTimer` 0.0)
          (for _array_element_3 (`self.LightsVariable`)
            (`/Game/Tom/Tom_Blueprints/BP_Lights.TurnLightOn` _array_element_3))
          (for _array_element_4 (`self.ArrayOfMannequinnes`)
            (set `/Game/Sharan/Blueprints/RBP_Mannequine1.LightsOn` true _array_element_4)))))))

(event `EventGraphBeginPlay`)

(event `EventGraphOnTick`
  (params (DeltaTime :type "Float (double-precision)"))
  (if (`self.InBadPlace`)
    (set `self.TimerForEvents` (+ DeltaTime (`self.TimerForEvents`)))
    (if (>= (`self.TimerForEvents`) (`KismetMathLibrary.RandomFloatInRange` 60.0 80.0))
      (set `self.TimerForEvents` 0.0)
      (`KismetSystemLibrary.PrintString` "Event GOOOOOO"))))

(event `CallCameraFallEvent`
  (params (Camera :type "/Game/Tom/Tom_Blueprints/BP_FollowCamera Object Reference"))
  (`/Game/Tom/Tom_Blueprints/BP_FollowCamera.Fall` Camera))

(event `CallBallRollEvent`)

(event `CallSingleRedLightEvent`
  (params (Light :type "/Game/Tom/Tom_Blueprints/BP_Lights Object Reference"))
  (`/Game/Tom/Tom_Blueprints/BP_Lights.TurnLightRed` Light)
  (bind _returnvalue (`|CreateWidget` "/Game/Sharan/UI/WIG_CameraFilter.WIG_CameraFilter_C" (`GameplayStatics.GetPlayerController` 0)))
  (set `self.CameraFilterRef` _returnvalue)
  (`UserWidget.AddToViewport` _returnvalue 0)
  (`/Game/Sharan/UI/WIG_CameraFilter.GetReferences` _returnvalue self Light))

(event `CallShakeRacksEvent`
  (params (Racks :type "Array of /Game/Tom/Tom_Blueprints/BP_MovableRacks Object Reference")))

(event `CallCrunchSoundEvent`)

(event `CallLightFallEvent`
  (params (Light :type "/Game/Tom/Tom_Blueprints/BP_Lights Object Reference")))

(event `CallClothesFallEvent`
  (params (Cloths :type "/Game/Tom/Tom_Blueprints/BP_CothesRandomiser Object Reference")))

(event `FinishSingleRedLightEvent`
  (`Widget.RemoveFromParent` (`self.CameraFilterRef`)))

(event `Spawn Coins`
  ;[1 1 1] SpawnsCoins
  (if (not (>= (`self.CoinCount`) 10))
    (bind _outactors (`GameplayStatics.GetAllActorsOfClass` "/Game/Tom/Tom_Blueprints/BP_CoinsSpawn.BP_CoinsSpawn_C"))
    (bind _success (`self.RandomSpawnObject` _outactors "/Game/Tom/Tom_Blueprints/BP_CoinPickup.BP_CoinPickup_C"))
    (if _success
      (`/Engine/EditorBlueprintResources/StandardMacros.IncrementInt` (`self.CoinCount`)
        (:`  `
          (`self.Spawn Coins`)))
      (else
        (`self.Spawn Coins`)))))

(event `Spawn Objectives`
  ;[1 1 1] SpawnsCoins
  (`self.SpawnDress`)
  (`self.SpawnSocks`)
  (`self.SpawnBoots`))

(event `SpawnDress`
  ;[1 1 1] SpawnsCoins
  (bind _outactors (`GameplayStatics.GetAllActorsOfClass` "/Game/Tom/Tom_Blueprints/BP_DressSpawn.BP_DressSpawn_C"))
  (bind (_success _spawnedobjectdetails) (`self.RandomSpawnObject` _outactors "/Game/Sharan/Blueprints/BP_Objectives.BP_Objectives_C"))
  (if _success
    (bind _objectiveref (message `/Game/Tom/Tom_Blueprints/BPI_GetObjectiveRef.GetObjectiveRef` _spawnedobjectdetails))
    (`/Engine/EditorBlueprintResources/StandardMacros.IsValid` _objectiveref
      (:`Is Valid`
        (set `/Game/Tom/Tom_Blueprints/BP_PickupBase.MeshToUse` "/Game/Tom/ModelsAndTextures/clothes/Dress_PlaceHolder_/Dress.Dress" _objectiveref)
        (set `/Game/Tom/Tom_Blueprints/BP_PickupBase.MaterialToUse` "/Game/Tom/ModelsAndTextures/clothes/Dress_PlaceHolder_/Material5266224.Material5266224" _objectiveref)
        (`/Game/Tom/Tom_Blueprints/BP_PickupBase.UpdateLooks` _objectiveref))
      (:`Is Not Valid`
        (`self.SpawnDress`)))
    (else
      (`self.SpawnDress`))))

(event `SpawnSocks`
  ;[1 1 1] SpawnsCoins
  (bind _outactors (`GameplayStatics.GetAllActorsOfClass` "/Game/Tom/Tom_Blueprints/BP_SocksSpawn.BP_SocksSpawn_C"))
  (bind (_success _spawnedobjectdetails) (`self.RandomSpawnObject` _outactors "/Game/Sharan/Blueprints/BP_Objectives.BP_Objectives_C"))
  (if _success
    (bind _objectiveref (message `/Game/Tom/Tom_Blueprints/BPI_GetObjectiveRef.GetObjectiveRef` _spawnedobjectdetails))
    (`/Engine/EditorBlueprintResources/StandardMacros.IsValid` _objectiveref
      (:`Is Valid`
        (set `/Game/Tom/Tom_Blueprints/BP_PickupBase.MeshToUse` "/Game/Tom/ModelsAndTextures/clothes/Socks/SM_Socks.SM_Socks" _objectiveref)
        (set `/Game/Tom/Tom_Blueprints/BP_PickupBase.MaterialToUse` "/Game/Tom/ModelsAndTextures/clothes/Socks/standardSurface1.standardSurface1" _objectiveref)
        (`/Game/Tom/Tom_Blueprints/BP_PickupBase.UpdateLooks` _objectiveref))
      (:`Is Not Valid`
        (`self.SpawnSocks`)))
    (else
      (`self.SpawnSocks`))))

(event `SpawnBoots`
  ;[1 1 1] SpawnsCoins
  (bind _outactors (`GameplayStatics.GetAllActorsOfClass` "/Game/Tom/Tom_Blueprints/BP_BootsSpawn.BP_BootsSpawn_C"))
  (bind (_success _spawnedobjectdetails) (`self.RandomSpawnObject` _outactors "/Game/Sharan/Blueprints/BP_Objectives.BP_Objectives_C"))
  (if _success
    (bind _objectiveref (message `/Game/Tom/Tom_Blueprints/BPI_GetObjectiveRef.GetObjectiveRef` _spawnedobjectdetails))
    (`/Engine/EditorBlueprintResources/StandardMacros.IsValid` _objectiveref
      (:`Is Valid`
        (set `/Game/Tom/Tom_Blueprints/BP_PickupBase.MeshToUse` "/Game/Tom/ModelsAndTextures/clothes/Boots/SM_Boots.SM_Boots" _objectiveref)
        (set `/Game/Tom/Tom_Blueprints/BP_PickupBase.MaterialToUse` "/Game/Tom/ModelsAndTextures/clothes/Boots/standardSurface2.standardSurface2" _objectiveref)
        (`/Game/Tom/Tom_Blueprints/BP_PickupBase.UpdateLooks` _objectiveref))
      (:`Is Not Valid`
        (`self.SpawnBoots`)))
    (else
      (`self.SpawnBoots`))))

(fn `GetGameModeInterface`
  (returns (GameModeRef :type "/Game/Tom/Tom_Blueprints/BP_GM_Level1 Object Reference"))
  (return self))

(fn `GetObjectiveRef`
  (returns (ObjectiveRef :type "/Game/Sharan/Blueprints/BP_Objectives Object Reference"))
  (return null))

(fn `RandomSpawnObject`
  (params (ArrayOfSpawnPoints :type "Array of Actor Object Reference") (ActorTypeToSpawn :type "Actor Class Reference"))
  (returns (Success :type Boolean) (SpawnedObjectDetails :type "Actor Object Reference"))
  (locals (RandomInt :type Integer :default 0))
  (bind _output (`|GetArrayItem` ArrayOfSpawnPoints (`local.RandomInt`)))
  (set `local.RandomInt` (`KismetMathLibrary.RandomIntegerInRange` 0 (- (`KismetArrayLibrary.Array_Length` ArrayOfSpawnPoints) 1)))
  (`/Engine/EditorBlueprintResources/StandardMacros.IsValid` _output
    (:`Is Valid`
      (bind _returnvalue (`|SpawnActorFromClass` ActorTypeToSpawn (`KismetMathLibrary.MakeTransform` (`self.K2_GetActorLocation` _output)) "Undefined" "MultiplyWithRoot" null null))
      (`self.K2_DestroyActor` _output)
      (return true _returnvalue))
    (:`Is Not Valid`
      (return false null))))

(fn `UserConstructionScript`)