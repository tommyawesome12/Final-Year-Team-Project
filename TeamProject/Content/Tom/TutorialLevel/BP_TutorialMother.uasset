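; Tutorial level pawn for the mother character, which walks to scripted spots on demand.
; Five custom events, MoveToLocation1 to 5, each issue an AI Move To on itself toward a hard-coded world position.
; The events are independent, with no chaining or completion handling, and nothing in this graph triggers them apart from an unreachable call to MoveToLocation4.
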(event `MoveToLocation1`
  (`|AIMoveTo` self (3667.993343 3667.993343 0.0) null))

(event `MoveToLocation2`
  (`|AIMoveTo` self (3915.934232 1879.779879 143.320439) null))

(event `MoveToLocation3`
  (`|AIMoveTo` self (2855.618657 1361.25042 143.320439) null))

(event `MoveToLocation4`
  (`|AIMoveTo` self (1150.445931 715.0 143.320439) null))

(event `MoveToLocation5`
  (`|AIMoveTo` self (621.053003 335.517794 143.320439) null))

(fn `UserConstructionScript`)