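; BP_CoinTutorial is a collectible coin for the tutorial level.
; Its TutorialInteract event increments the Coins count on the passed player reference, then destroys the actor.
; A MakeVisible event unhides the Sphere1 component in game, without propagating to its children.
; The construction script runs the parent's script, then sets MeshToUse to the machine coin mesh.
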(event `/Game/Tom/TutorialLevel/BPI_TutorialInteract.TutorialInteract`
  (params (PlayerRef :type "/Game/Tom/TutorialLevel/BP_Tuorial Object Reference"))
  (`/Engine/EditorBlueprintResources/StandardMacros.IncrementInt` (`/Game/Tom/TutorialLevel/BP_Tuorial.Coins` PlayerRef)
    (:`  `
      (`self.K2_DestroyActor`))))

(event `MakeVisible`
  (`SceneComponent.SetHiddenInGame` (`self.Sphere1`) false false))

(fn `UserConstructionScript`
  (`parent.UserConstructionScript`)
  (set `self.MeshToUse` "/Game/Tom/ModelsAndTextures/Coin/SM_MachineCoin__1_.SM_MachineCoin__1_"))