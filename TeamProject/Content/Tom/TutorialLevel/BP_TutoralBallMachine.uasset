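; Tutorial-level ball machine that the player pays a coin to use, restoring Sanity.
; On BeginPlay it casts the game mode to BP_GM_Tutorial and caches the reference.
; TutorialInteract checks that the player has coins, deducts one, sets Sanity to full and calls the game mode's AfterBallDialogue to continue the tutorial.
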(event `self.ReceiveBeginPlay`
  (bind _asbp_gm_tutorial (cast `/Game/Tom/TutorialLevel/BP_GM_Tutorial` (`GameplayStatics.GetGameMode`)))
  (set `self.GameModeRef` _asbp_gm_tutorial))

(event `/Game/Tom/TutorialLevel/BPI_TutorialInteract.TutorialInteract`
  (params (PlayerRef :type "/Game/Tom/TutorialLevel/BP_Tuorial Object Reference"))
  (bind _coins (`/Game/Tom/TutorialLevel/BP_Tuorial.Coins` PlayerRef))
  (if (> _coins 0)
    (`/Engine/EditorBlueprintResources/StandardMacros.DecrementInt` _coins
      (:`  `
        (set `/Game/Tom/TutorialLevel/BP_Tuorial.Sanity` 1.0 PlayerRef)
        (`/Game/Tom/TutorialLevel/BP_GM_Tutorial.AfterBallDialogue` (`self.GameModeRef`))))))

(fn `UserConstructionScript`)