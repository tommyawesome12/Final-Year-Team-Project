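; Tutorial level game mode that scripts the story of Connor and his mom in a store, teaching that mannequins stay still while watched.
; BeginPlay caches the player and mother actor and starts the opening dialogue.
; Staged events show timed HUD lines, reveal the coin, remove blockers and send the mother to successive locations.
; Later stages await external calls; the one-shot till scene ends by opening JohnLevel.
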(event `self.ReceiveBeginPlay`
  (bind _asbp_tuorial (cast `/Game/Tom/TutorialLevel/BP_Tuorial` (`GameplayStatics.GetPlayerCharacter` 0)))
  (set `self.PlayerCharacterRef` _asbp_tuorial)
  (`KismetSystemLibrary.DelayUntilNextTick`)
  (`self.StartDialogue`)
  (bind _returnvalue (`GameplayStatics.GetActorOfClass` "/Game/Tom/TutorialLevel/BP_TutorialMother.BP_TutorialMother_C"))
  (set `self.MotherRef` _returnvalue))

(event `StartDialogue`
  (bind _hudref (`/Game/Tom/TutorialLevel/BP_Tuorial.HUDRef` (`self.PlayerCharacterRef`)))
  (`/Game/Tom/TutorialLevel/Widgets/BP_TutorialHUD.SetBorderColour` _hudref)
  (set `/Game/Tom/TutorialLevel/Widgets/BP_TutorialHUD.Text` "Mom: I’m so proud of you for coming with me and trying to get over your fear of mannequins just remember what I said, if u look at them, they wont seem so scary to you anymore." _hudref)
  (`KismetSystemLibrary.Delay` 5.0)
  (`/Game/Tom/TutorialLevel/BP_TutorialMother.MoveToLocation1` (`self.MotherRef`)))

(event `BeforeBallDialogue`
  (bind _hudref (`/Game/Tom/TutorialLevel/BP_Tuorial.HUDRef` (`self.PlayerCharacterRef`)))
  (`/Game/Tom/TutorialLevel/Widgets/BP_TutorialHUD.SetBorderColour` _hudref)
  (set `/Game/Tom/TutorialLevel/Widgets/BP_TutorialHUD.Text` "Mom: Look Connor its that ball machine you like, here's a quarter put it in the machine and get a bouncy ball, I know how happy they make you." _hudref)
  (bind _returnvalue (`GameplayStatics.GetActorOfClass` "/Game/Tom/TutorialLevel/BP_CoinTutorial.BP_CoinTutorial_C"))
  (`/Game/Tom/TutorialLevel/BP_CoinTutorial.MakeVisible` _returnvalue)
  (`KismetSystemLibrary.Delay` 5.0)
  (`/Game/Tom/TutorialLevel/Widgets/BP_TutorialHUD.ResetToBlank` _hudref))

(event `AfterBallDialogue`
  (bind _hudref (`/Game/Tom/TutorialLevel/BP_Tuorial.HUDRef` (`self.PlayerCharacterRef`)))
  (`/Game/Tom/TutorialLevel/Widgets/BP_TutorialHUD.SetBorderColour` _hudref)
  (set `/Game/Tom/TutorialLevel/Widgets/BP_TutorialHUD.Text` "Mom: See are you feeling better now? Lets go window shopping for a bit before we decide what we should get." _hudref)
  (`KismetSystemLibrary.Delay` 5.0)
  (`/Game/Tom/TutorialLevel/Widgets/BP_TutorialHUD.ResetToBlank` _hudref)
  (bind _returnvalue (`GameplayStatics.GetActorOfClass` "/Game/Tom/TutorialLevel/BP_BallBlocker.BP_BallBlocker_C"))
  (`self.K2_DestroyActor` _returnvalue)
  (`/Game/Tom/TutorialLevel/BP_TutorialMother.MoveToLocation2` (`self.MotherRef`)))

(event `BeforeDress`
  (bind _hudref (`/Game/Tom/TutorialLevel/BP_Tuorial.HUDRef` (`self.PlayerCharacterRef`)))
  (`/Game/Tom/TutorialLevel/Widgets/BP_TutorialHUD.SetBorderColour` _hudref)
  (set `/Game/Tom/TutorialLevel/Widgets/BP_TutorialHUD.Text` "Mom: that dress looks so pretty I might add it to the list what do you think Connor?" _hudref)
  (`KismetSystemLibrary.Delay` 5.0)
  (set `/Game/Tom/TutorialLevel/Widgets/BP_TutorialHUD.Text` "Connor: I think it looks nice! should we grab it now?" _hudref)
  (`KismetSystemLibrary.Delay` 5.0)
  (set `/Game/Tom/TutorialLevel/Widgets/BP_TutorialHUD.Text` "Mom: No don't worry we can get it later, just want to look around first, need to find something for you, your sister and your dad now." _hudref)
  (`KismetSystemLibrary.Delay` 5.0)
  (bind _returnvalue (`GameplayStatics.GetActorOfClass` "/Game/Tom/TutorialLevel/BP_DressBlocker.BP_DressBlocker_C"))
  (`self.K2_DestroyActor` _returnvalue)
  (`/Game/Tom/TutorialLevel/BP_TutorialMother.MoveToLocation3` (`self.MotherRef`)))

(event `BeforeMannequinne`
  (bind _hudref (`/Game/Tom/TutorialLevel/BP_Tuorial.HUDRef` (`self.PlayerCharacterRef`)))
  (`/Game/Tom/TutorialLevel/Widgets/BP_TutorialHUD.SetBorderColour` _hudref)
  (set `/Game/Tom/TutorialLevel/Widgets/BP_TutorialHUD.Text` "Connor: Are you sure it wont move mom?" _hudref)
  (`KismetSystemLibrary.Delay` 5.0)
  (set `/Game/Tom/TutorialLevel/Widgets/BP_TutorialHUD.Text` "Mom: I promise look, while you're looking at it its not moving at all is it? This is a normal store they can't hurt you here." _hudref)
  (`KismetSystemLibrary.Delay` 5.0)
  (`/Game/Tom/TutorialLevel/Widgets/BP_TutorialHUD.ResetToBlank` _hudref)
  (`/Game/Tom/TutorialLevel/BP_TutorialMother.MoveToLocation4` (`self.MotherRef`)))

(event `BeforeTill`
  (bind _hudref (`/Game/Tom/TutorialLevel/BP_Tuorial.HUDRef` (`self.PlayerCharacterRef`)))
  (`/Engine/EditorBlueprintResources/StandardMacros.DoOnce` false
    (:`Completed`
      (`/Game/Tom/TutorialLevel/BP_TutorialMother.MoveToLocation5` (`self.MotherRef`))
      (`/Game/Tom/TutorialLevel/Widgets/BP_TutorialHUD.SetBorderColour` _hudref)
      (set `/Game/Tom/TutorialLevel/Widgets/BP_TutorialHUD.Text` "Mom: Wait is that Rachel working? Connor would you mind going and collecting the things on the list?" _hudref)
      (`KismetSystemLibrary.Delay` 5.0)
      (set `/Game/Tom/TutorialLevel/Widgets/BP_TutorialHUD.Text` "Connor: I don't mind but what about the mannequins" _hudref)
      (`KismetSystemLibrary.Delay` 5.0)
      (set `/Game/Tom/TutorialLevel/Widgets/BP_TutorialHUD.Text` "Mom: Just remember what I've told you, when you look at them you can see that they won't move" _hudref)
      (`KismetSystemLibrary.Delay` 5.0)
      (`GameplayStatics.OpenLevelBySoftObjectPtr` "/Game/John/JohnLevel.JohnLevel"))))

(fn `UserConstructionScript`)